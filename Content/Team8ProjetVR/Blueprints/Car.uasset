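; Player car actor for a VR driving game that carries the player pawn and steers sideways from a steering wheel.
; BeginPlay shows the UI, attaches the pawn and caches the wheel component from a child actor.
; Tick slides the car along its right vector using wheel input once the GameManager starts it, while a Timeline optionally bobs its height.
; Ending an overlap signals death, plays a crash sound and reloads the level after a delay.
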(event `self.ReceiveBeginPlay`
  (bind (_returnvalue_x _returnvalue_y) (`KismetMathLibrary.BreakVector` (`self.K2_GetActorLocation`)))
  (bind (_baseactorlocation_x _baseactorlocation_y _baseactorlocation_z) (`KismetMathLibrary.BreakVector` (`self.BaseActorLocation`)))
  (`|ExecutionSequence`
    (:`then_0`
      (bind _returnvalue (`|CreateWidget` "/Game/Team8ProjetVR/Widgets/UI.UI_C"))
      (`UserWidget.AddToViewport` _returnvalue 0))
    (:`then_1`
      (`self.K2_AttachToActor` (`GameplayStatics.GetPlayerPawn` 0) self "None" "KeepWorld" "KeepWorld" "KeepWorld" true)
      (bind _assteering_wheel (cast `/Game/Project/BP/Grabbable/SteeringWheel` (`ChildActorComponent.ChildActor` (`self.Wheel`))))
      (set `self.SteerinWheel` (`/Game/Project/BP/Grabbable/SteeringWheel.SteeringWheel` _assteering_wheel))
      (set `self.BaseActorLocation` (`self.K2_GetActorLocation`))
      (bind (_direction _repeatingcarbobble) (`Timeline|Timeline`)
        (:`Update`
          (if (`self.VehicleBobble`)
            (`self.K2_SetActorLocation` (`KismetMathLibrary.MakeVector` _returnvalue_x _returnvalue_y (+ _repeatingcarbobble _baseactorlocation_z)))))))))

(event `self.ReceiveActorEndOverlap`
  (params (OtherActor :type "Actor Object Reference"))
  (`GameManager.OnDie` (subsystem `GameManager`))
  (`GameplayStatics.PlaySound2D` "/Game/Team8ProjetVR/Sound/SFX/Voiture/SFX_GameOver_CarCrash.SFX_GameOver_CarCrash" 1.0 1.0 4.0 null null false)
  (`KismetSystemLibrary.Delay` 10.0)
  (bind _returnvalue (`GameplayStatics.GetCurrentLevelName` true))
  (`GameplayStatics.OpenLevel` (`KismetStringLibrary.Conv_StringToName` _returnvalue)))

(event `self.ReceiveTick`
  (params (DeltaSeconds :type "Float (single-precision)"))
  (if (`GameManager.IsCarStarted` (subsystem `GameManager`))
    (`self.K2_AddActorWorldOffset` (* (`SceneComponent.GetRightVector` (`self.Car`)) (* DeltaSeconds (* (`self.Speed`) (* (`SteeringWheelComponent.DriveInputXValue` (`self.SteerinWheel`)) -1.0)))))))

(fn `UserConstructionScript`)